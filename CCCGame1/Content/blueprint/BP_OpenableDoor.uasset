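; Openable door actor that swings open and shut around its yaw axis, with opening and closing sounds.
; Open and close events from the OpenDoor component play or reverse a timeline that lerps the actor's relative rotation.
; Timeline event tracks trigger the sounds, and a shared PlayMusic flag blocks new door commands and sounds during a short cooldown after each sound.
; BeginPlay calls CFunction on the component.
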(event OnCloseDoor(OpenDoor)
  (bind _returnvalue (Transformation|GetActorLocation))
  (if (Variables|Default|GetplayMusic)
    (bind _opendooralpha (Timeline|tlOpenDoor Reverse)
      (:Update
        (Transformation|SetActorRelativeRotation (Math|Rotator|MakeRotator 0.0 0.0 (Math|Float|Lerp 0.0 -75.0 _opendooralpha))))
      (:playOpenSound
        (if (Variables|Default|GetplayMusic)
          (Variables|Default|SetplayMusic false)
          (Audio|PlaySoundatLocation "/Game/openDoor.openDoor" _returnvalue)
          (Utilities|FlowControl|Delay 2.0 :!label _label)
          (Variables|Default|SetplayMusic true)))
      (:playCloseSound
        (if (Variables|Default|GetplayMusic)
          (Variables|Default|SetplayMusic false)
          (Audio|PlaySoundatLocation "/Game/closeDoor.closeDoor" _returnvalue)
          (goto _label))))))

(event OnOpenDoor(OpenDoor)
  (bind _returnvalue (Transformation|GetActorLocation))
  (if (Variables|Default|GetplayMusic)
    (bind _opendooralpha (Timeline|tlOpenDoor Play)
      (:Update
        (Transformation|SetActorRelativeRotation (Math|Rotator|MakeRotator 0.0 0.0 (Math|Float|Lerp 0.0 -75.0 _opendooralpha))))
      (:playOpenSound
        (if (Variables|Default|GetplayMusic)
          (Variables|Default|SetplayMusic false)
          (Audio|PlaySoundatLocation "/Game/openDoor.openDoor" _returnvalue)
          (Utilities|FlowControl|Delay 2.0 :!label _label)
          (Variables|Default|SetplayMusic true)))
      (:playCloseSound
        (if (Variables|Default|GetplayMusic)
          (Variables|Default|SetplayMusic false)
          (Audio|PlaySoundatLocation "/Game/closeDoor.closeDoor" _returnvalue)
          (goto _label))))))

(event EventBeginPlay
  (Class|OpenDoor|CFunction (Variables|Default|GetOpenDoor)))

(event Collision|EventActorBeginOverlap
  (params (OtherActor :type Actor%20Object%20Reference)))

(event EventTick
  (params (DeltaSeconds :type Float%20%28single-precision%29)))

(fn ConstructionScript)